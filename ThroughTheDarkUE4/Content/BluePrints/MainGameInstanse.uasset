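; Game instance that serves as the central hub for a puzzle game's UI and progression state.
; Events lazily create and cache menu, inventory, document, code-lock and ending widgets, toggling pause and input mode as needed.
; Document pickups and reads, code entry and a six-statue check drive flags and call level actors found by class to open paths and enable the door or mirror ending.
; New game shows a loading screen, opens Starter_Room and resets progress.
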(event Custom|Show%20Options%20Menu
  ;[1 1 1] Вызов меню настроек
  (Utilities|IsValid (Variables|Widgets|GetOptionsMenuWB)
    (:Is%20Valid
      _)
    (:Is%20Not%20Valid
      (bind _returnvalue (UserInterface|CreateWidget "/Game/UI/Menus/OptionsMenuWB.OptionsMenuWB_C" (Game|GetPlayerController 0)))
      (Variables|Widgets|SetOptionsMenuWB _returnvalue)))
  (UserInterface|Viewport|AddtoViewport (Variables|Widgets|GetOptionsMenuWB) 0))

(event Custom|Show%20Main%20Menu
  (bind _returnvalue (Game|GetPlayerController 0))
  ;[1 1 1] Вызов главного меню
  (Utilities|IsValid (Variables|Widgets|GetMainMenuWB)
    (:Is%20Valid
      _)
    (:Is%20Not%20Valid
      (bind _returnvalue_2 (UserInterface|CreateWidget "/Game/UI/Menus/MainMenuWB.MainMenuWB_C" _returnvalue))
      (Variables|Widgets|SetMainMenuWB _returnvalue_2)))
  (UserInterface|Viewport|AddtoViewport (Variables|Widgets|GetMainMenuWB) 0)
  (Variables|/Script/Engine.PlayerController|SetbShowMouseCursor _returnvalue true)
  (Input|SetInputModeUIOnly _returnvalue (Variables|Widgets|GetMainMenuWB) "LockInFullscreen"))

(event Custom|Pause%20Menu%20Resume
  (bind _returnvalue (Game|GetPlayerController 0))
  ;[1 1 1] Вернуться в игру из паузы
  (Widget|RemovefromParent (Variables|Widgets|GetPauseMenuWB))
  (Game|SetGamePaused false)
  (Input|SetInputModeGameOnly _returnvalue)
  (Variables|/Script/Engine.PlayerController|SetbShowMouseCursor _returnvalue false))

(event Custom|FindForthDocument
  ;[1 1 1] Четвертый документ
  ;;[1 1 1] Подбор четвертого документа
  (Utilities|IsValid (Variables|Widgets|GetInventoryWB)
    (:Is%20Valid
      _)
    (:Is%20Not%20Valid
      (bind _returnvalue (UserInterface|CreateWidget "/Game/UI/Documents/Inventory.Inventory_C" (Game|GetPlayerController 0)))
      (Variables|Widgets|SetInventoryWB _returnvalue)))
  (Default|UnlockForthDocument (Variables|Widgets|GetInventoryWB))
  (Audio|PlaySound2D "/Game/Audio/InGame/PickDocument.PickDocument" 1.0 1.0 0.0 0 0))

(event Custom|Show%20Help%20Menu
  ;[1 1 1] Открыть меню справки
  (Utilities|IsValid (Variables|Widgets|GetHelpMenuWB)
    (:Is%20Valid
      _)
    (:Is%20Not%20Valid
      (bind _returnvalue (UserInterface|CreateWidget "/Game/UI/Menus/HelpMenuWB.HelpMenuWB_C" (Game|GetPlayerController 0)))
      (Variables|Widgets|SetHelpMenuWB _returnvalue)))
  (UserInterface|Viewport|AddtoViewport (Variables|Widgets|GetHelpMenuWB) 0))

(event Custom|ReturnFromForthDocument
  ;[1 1 1] Четвертый документ
  ;;[1 1 1] Возвращение из четвертого документа
  (Widget|RemovefromParent (Variables|Widgets|GetForthDocumentWB)))

(event Custom|ShowForthDocument
  ;[1 1 1] Четвертый документ
  ;;[1 1 1] Открытие четвертого документа
  (Utilities|IsValid (Variables|Widgets|GetForthDocumentWB)
    (:Is%20Valid
      _)
    (:Is%20Not%20Valid
      (bind _returnvalue (UserInterface|CreateWidget "/Game/UI/Documents/ForthDocument.ForthDocument_C" (Game|GetPlayerController 0)))
      (Variables|Widgets|SetForthDocumentWB _returnvalue)))
  (bind _outactors (Actor|GetAllActorsOfClass "/Game/BluePrints/Triggers/EndGameDoor.EndGameDoor_C"))
  (Default|EnableEvent _outactors)
  (bind _outactors_2 (Actor|GetAllActorsOfClass "/Game/BluePrints/Triggers/EndGameMirrow.EndGameMirrow_C"))
  (Default|EnableEvent _outactors_2)
  (UserInterface|Viewport|AddtoViewport (Variables|Widgets|GetForthDocumentWB) 0)
  (bind _outactors_3 (Actor|GetAllActorsOfClass "/Game/BluePrints/Triggers/EndGameMirrow.EndGameMirrow_C"))
  (Default|EditMaterial _outactors_3))

(event Custom|OpenCodeDoor
  (bind _returnvalue (Game|GetPlayerController 0))
  ;[1 1 1] Код от двери
  ;;[1 1 1] Открытие модуля для кода двери
  (if (not (Variables|Default|GetIsDoorOpened))
    (if (Variables|Default|GetIsFirstDocumentTaken)
      (Utilities|IsValid (Variables|Widgets|GetCodeDoorWB)
        (:Is%20Valid
          _)
        (:Is%20Not%20Valid
          (bind _returnvalue_2 (UserInterface|CreateWidget "/Game/UI/CodeInput/CodeMenu.CodeMenu_C" _returnvalue))
          (Variables|Widgets|SetCodeDoorWB _returnvalue_2)))
      (UserInterface|Viewport|AddtoViewport (Variables|Widgets|GetCodeDoorWB) 0)
      (Input|SetInputModeUIOnly _returnvalue (Variables|Widgets|GetCodeDoorWB) "DoNotLock")
      (Game|SetGamePaused true)
      (Variables|/Script/Engine.PlayerController|SetbShowMouseCursor _returnvalue true))))

(event Custom|Return%20From%20Inventory
  (bind _returnvalue (Game|GetPlayerController 0))
  ;[1 1 1] Вернуться в игру из инвентаря
  (Widget|RemovefromParent (Variables|Widgets|GetInventoryWB))
  (Game|SetGamePaused false)
  (Input|SetInputModeGameOnly _returnvalue)
  (Variables|/Script/Engine.PlayerController|SetbShowMouseCursor _returnvalue false))

(event Custom|InputRightCode
  ;[1 1 1] Код от двери
  ;;[1 1 1] Ввод правильного кода
  (bind _outactors (Actor|GetAllActorsOfClass "/Game/BluePrints/Doors/Door_Blueprint.Door_Blueprint_C"))
  (Default|SetDoorEnabled _outactors)
  (Variables|Default|SetIsDoorOpened true)
  (CallFunction|ReturnfromCodeDoor))

(event Custom|FindFirstDocument
  ;[1 1 1] Первый документ
  ;;[1 1 1] Подбор первого документа
  (Utilities|IsValid (Variables|Widgets|GetInventoryWB)
    (:Is%20Valid
      _)
    (:Is%20Not%20Valid
      (bind _returnvalue (UserInterface|CreateWidget "/Game/UI/Documents/Inventory.Inventory_C" (Game|GetPlayerController 0)))
      (Variables|Widgets|SetInventoryWB _returnvalue)))
  (Default|UnlockFirstDocument (Variables|Widgets|GetInventoryWB))
  (bind _outactors (Actor|GetAllActorsOfClass "/Game/BluePrints/Triggers/LightFromFirstDocument.LightFromFirstDocument_C"))
  (Default|TurnonLight _outactors)
  (Variables|Default|SetIsFirstDocumentTaken true)
  (Audio|PlaySound2D "/Game/Audio/InGame/PickDocument.PickDocument" 1.0 1.0 0.0 0 0))

(event Custom|ReturnFromFirstDocument
  ;[1 1 1] Первый документ
  ;;[1 1 1] Возвращение из первого документа
  (Widget|RemovefromParent (Variables|Widgets|GetFirstDocumentWB)))

(event Custom|CreateNewGame
  (bind _returnvalue (Game|GetPlayerController 0))
  ;[1 1 1] Создать новую игру
  (Variables|/Script/Engine.PlayerController|SetbShowMouseCursor _returnvalue false)
  (Input|SetInputModeGameOnly _returnvalue)
  (CallFunction|ShowLoadingScreen)
  (Utilities|FlowControl|Delay 4.0)
  (Widget|RemovefromParent (Variables|Widgets|GetLoadingScreenWB))
  (Game|OpenLevel(byObjectReference) "/Game/FirstPersonBP/Maps/Starter_Room.Starter_Room")
  (CallFunction|InitializeNewGame))

(event Custom|ShowFirstDocument
  ;[1 1 1] Первый документ
  ;;[1 1 1] Открытие первого документа
  (Utilities|IsValid (Variables|Widgets|GetFirstDocumentWB)
    (:Is%20Valid
      _)
    (:Is%20Not%20Valid
      (bind _returnvalue (UserInterface|CreateWidget "/Game/UI/Documents/FirstDocument.FirstDocument_C" (Game|GetPlayerController 0)))
      (Variables|Widgets|SetFirstDocumentWB _returnvalue)))
  (UserInterface|Viewport|AddtoViewport (Variables|Widgets|GetFirstDocumentWB) 0))

(event Custom|DestroyMirrow
  ;[1 1 1] Уничтожение невидимой стены зеркала
  (if (and (Variables|Default|GetIsMirrowNotDestroyed) (Variables|Default|GetIsSecondDocumentTaken))
    (bind _outactors (Actor|GetAllActorsOfClass "/Game/BluePrints/Doors/Invisible_Mirrow_Blueprint.Invisible_Mirrow_Blueprint_C"))
    (Default|DestroyWallMirrow _outactors)
    (Variables|Default|SetIsMirrowNotDestroyed false)
    (Audio|PlaySound2D "/Game/Audio/InGame/BreakMirrow.BreakMirrow" 1.0 1.0 0.0 0 0)))

(event Custom|PlayAngelSound
  ;[1 1 1] Звук передвигания статуй
  (Audio|PlaySound2D "/Game/Audio/InGame/AngelAudio.AngelAudio" 1.0 1.0 0.0 0 0))

(event Custom|AllAngelsCorrect
  ;[1 1 1] Верное расположение всех статуй
  (bind _iscorrect (CallFunction|IsAllAngelsCorrect))
  (if _iscorrect
    (bind _outactors (Actor|GetAllActorsOfClass "/Game/BluePrints/Doors/InvisibleDoor_Blueprint.InvisibleDoor_Blueprint_C"))
    (Default|DestroyWallDoor _outactors)))

(event Custom|EndGameMirror
  (bind _returnvalue (Game|GetPlayerController 0))
  ;[1 1 1] Конец игры: зеркало
  ;;[1 1 1] Вызов конца игры при выборе зеркала
  (Utilities|IsValid (Variables|Widgets|GetEndGameMirrorWB)
    (:Is%20Valid
      _)
    (:Is%20Not%20Valid
      (bind _returnvalue_2 (UserInterface|CreateWidget "/Game/UI/Menus/EndGameMirrowWB.EndGameMirrowWB_C" _returnvalue))
      (Variables|Widgets|SetEndGameMirrorWB _returnvalue_2)))
  (UserInterface|Viewport|AddtoViewport (Variables|Widgets|GetEndGameMirrorWB) 0)
  (Input|SetInputModeUIOnly _returnvalue (Variables|Widgets|GetEndGameMirrorWB) "DoNotLock")
  (Game|SetGamePaused true)
  (Variables|/Script/Engine.PlayerController|SetbShowMouseCursor _returnvalue true)
  (Audio|PlaySound2D "/Game/Audio/InGame/EndGame_Cue.EndGame_Cue" 1.0 1.0 0.0 0 0))

(event Custom|ReturnFromEndGameMirror
  ;[1 1 1] Конец игры: зеркало
  ;;[1 1 1] Вернуться из конца игры зеркала
  (Widget|RemovefromParent (Variables|Widgets|GetEndGameMirrorWB))
  (Game|OpenLevel(byObjectReference) "/Game/FirstPersonBP/Maps/MainMenu.MainMenu"))

(event Custom|EndGameDoor
  (bind _returnvalue (Game|GetPlayerController 0))
  ;[1 1 1] Конец игры: Дверь
  ;;[1 1 1] Вызов конца игры при выборе двери
  (Utilities|IsValid (Variables|Widgets|GetEndGameDoorWB)
    (:Is%20Valid
      _)
    (:Is%20Not%20Valid
      (bind _returnvalue_2 (UserInterface|CreateWidget "/Game/UI/Menus/EndGameDoorWB.EndGameDoorWB_C" _returnvalue))
      (Variables|Widgets|SetEndGameDoorWB _returnvalue_2)))
  (UserInterface|Viewport|AddtoViewport (Variables|Widgets|GetEndGameDoorWB) 0)
  (Input|SetInputModeUIOnly _returnvalue (Variables|Widgets|GetEndGameDoorWB) "DoNotLock")
  (Game|SetGamePaused true)
  (Variables|/Script/Engine.PlayerController|SetbShowMouseCursor _returnvalue true)
  (Audio|PlaySound2D "/Game/Audio/InGame/EndGame_Cue.EndGame_Cue" 1.0 1.0 0.0 0 0))

(event Custom|Initialize%20New%20Game
  ;[1 1 1] Инициализация новой игры
  (Variables|Default|SetIsDoorOpened false)
  (Variables|Default|SetIsFirstDocumentTaken false)
  (Variables|Default|SetIsSecondDocumentTaken false)
  (Variables|Default|SetIsMirrowNotDestroyed true)
  (Variables|Default|SetIsThirdDocumentRead false)
  (Variables|Default|SetAngelsPositions (Variables|Default|GetAngels%20Positions%20Default))
  (Utilities|IsValid (Variables|Widgets|GetInventoryWB)
    (:Is%20Valid
      _)
    (:Is%20Not%20Valid
      (bind _returnvalue (UserInterface|CreateWidget "/Game/UI/Documents/Inventory.Inventory_C" (Game|GetPlayerController 0)))
      (Variables|Widgets|SetInventoryWB _returnvalue)))
  (Default|ClearDocuments (Variables|Widgets|GetInventoryWB)))

(event Custom|ReturnFromDoorEndGame
  ;[1 1 1] Конец игры: Дверь
  ;;[1 1 1] Вернуться из конца игры двери
  (Widget|RemovefromParent (Variables|Widgets|GetEndGameDoorWB))
  (Game|OpenLevel(byObjectReference) "/Game/FirstPersonBP/Maps/MainMenu.MainMenu"))

(event Custom|Show%20Loading%20Screen
  ;[1 1 1] Показ экрана загрузки
  (Utilities|IsValid (Variables|Widgets|GetLoadingScreenWB)
    (:Is%20Valid
      _)
    (:Is%20Not%20Valid
      (bind _returnvalue (UserInterface|CreateWidget "/Game/UI/Menus/LoadingScreen.LoadingScreen_C" (Game|GetPlayerController 0)))
      (Variables|Widgets|SetLoadingScreenWB _returnvalue)))
  (UserInterface|Viewport|AddtoViewport (Variables|Widgets|GetLoadingScreenWB) 0))

(event Custom|PauseMenu:%20Show%20OptionsMenu
  ;[1 1 1] Вызов меню настроек из меню паузы
  (Widget|RemovefromParent (Variables|Widgets|GetPauseMenuWB))
  (Utilities|IsValid (Variables|Widgets|GetPauseOptionsMenuWB)
    (:Is%20Valid
      _)
    (:Is%20Not%20Valid
      (bind _returnvalue (UserInterface|CreateWidget "/Game/UI/Menus/PauseMenuOptionsMenuWB.PauseMenuOptionsMenuWB_C" (Game|GetPlayerController 0)))
      (Variables|Widgets|SetPauseOptionsMenuWB _returnvalue)))
  (UserInterface|Viewport|AddtoViewport (Variables|Widgets|GetPauseOptionsMenuWB) 0))

(event Custom|PauseMenuOptionsMenu:%20Go%20to%20PauseMenu
  ;[1 1 1] Выход из меню настроек паузы в меню паузы
  (Widget|RemovefromParent (Variables|Widgets|GetPauseOptionsMenuWB))
  (UserInterface|Viewport|AddtoViewport (Variables|Widgets|GetPauseMenuWB) 0))

(event Custom|Show%20Pause%20Menu
  (bind _returnvalue (Game|GetPlayerController 0))
  ;[1 1 1] Вызов меню паузы
  (Utilities|IsValid (Variables|Widgets|GetPauseMenuWB)
    (:Is%20Valid
      _)
    (:Is%20Not%20Valid
      (bind _returnvalue_2 (UserInterface|CreateWidget "/Game/UI/Menus/PauseMenuWB.PauseMenuWB_C" _returnvalue))
      (Variables|Widgets|SetPauseMenuWB _returnvalue_2)))
  (UserInterface|Viewport|AddtoViewport (Variables|Widgets|GetPauseMenuWB) 0)
  (Input|SetInputModeUIOnly _returnvalue (Variables|Widgets|GetPauseMenuWB) "DoNotLock")
  (Game|SetGamePaused true)
  (Variables|/Script/Engine.PlayerController|SetbShowMouseCursor _returnvalue true))

(event Custom|FindSecondDocument
  ;[1 1 1] Второй документ
  ;;[1 1 1] Подбор второго документа
  (Utilities|IsValid (Variables|Widgets|GetInventoryWB)
    (:Is%20Valid
      _)
    (:Is%20Not%20Valid
      (bind _returnvalue (UserInterface|CreateWidget "/Game/UI/Documents/Inventory.Inventory_C" (Game|GetPlayerController 0)))
      (Variables|Widgets|SetInventoryWB _returnvalue)))
  (Default|UnlockSecondDocument (Variables|Widgets|GetInventoryWB))
  (Variables|Default|SetIsSecondDocumentTaken true)
  (Audio|PlaySound2D "/Game/Audio/InGame/PickDocument.PickDocument" 1.0 1.0 0.0 0 0))

(event Custom|ReturnFromSecondDocument
  ;[1 1 1] Второй документ
  ;;[1 1 1] Возвращение из второго документа
  (Widget|RemovefromParent (Variables|Widgets|GetSecondDocumentWB)))

(event Custom|ReturnFromCodeDoor
  (bind _returnvalue (Game|GetPlayerController 0))
  ;[1 1 1] Код от двери
  ;;[1 1 1] Вернуться в игру из ввода кода двери
  (Widget|RemovefromParent (Variables|Widgets|GetCodeDoorWB))
  (Game|SetGamePaused false)
  (Input|SetInputModeGameOnly _returnvalue)
  (Variables|/Script/Engine.PlayerController|SetbShowMouseCursor _returnvalue false))

(event Custom|ShowSecondDocument
  ;[1 1 1] Второй документ
  ;;[1 1 1] Открытие второго документа
  (Utilities|IsValid (Variables|Widgets|GetSecondDocumentWB)
    (:Is%20Valid
      _)
    (:Is%20Not%20Valid
      (bind _returnvalue (UserInterface|CreateWidget "/Game/UI/Documents/SecondDocument.SecondDocument_C" (Game|GetPlayerController 0)))
      (Variables|Widgets|SetSecondDocumentWB _returnvalue)))
  (UserInterface|Viewport|AddtoViewport (Variables|Widgets|GetSecondDocumentWB) 0))

(event Custom|FindThirdDocument
  ;[1 1 1] Третий документ
  ;;[1 1 1] Подбор третьего документа
  (Utilities|IsValid (Variables|Widgets|GetInventoryWB)
    (:Is%20Valid
      _)
    (:Is%20Not%20Valid
      (bind _returnvalue (UserInterface|CreateWidget "/Game/UI/Documents/Inventory.Inventory_C" (Game|GetPlayerController 0)))
      (Variables|Widgets|SetInventoryWB _returnvalue)))
  (Default|UnlockThirdDocument (Variables|Widgets|GetInventoryWB))
  (Audio|PlaySound2D "/Game/Audio/InGame/PickDocument.PickDocument" 1.0 1.0 0.0 0 0))

(event Custom|Return%20FromThirdDocument
  ;[1 1 1] Третий документ
  ;;[1 1 1] Возвращение из третьего документа
  (Widget|RemovefromParent (Variables|Widgets|GetThirdDocumentWB)))

(event Custom|ShowThirdDocument
  ;[1 1 1] Третий документ
  ;;[1 1 1] Открытие третьего документа
  (Utilities|IsValid (Variables|Widgets|GetThirdDocumentWB)
    (:Is%20Valid
      _)
    (:Is%20Not%20Valid
      (bind _returnvalue (UserInterface|CreateWidget "/Game/UI/Documents/ThirdDocument.ThirdDocument_C" (Game|GetPlayerController 0)))
      (Variables|Widgets|SetThirdDocumentWB _returnvalue)))
  (UserInterface|Viewport|AddtoViewport (Variables|Widgets|GetThirdDocumentWB) 0)
  (if (not (Variables|Default|GetIsThirdDocumentRead))
    (bind _outactors (Actor|GetAllActorsOfClass "/Game/BluePrints/Doors/DestroyingDoor.DestroyingDoor_C"))
    (Default|DestroyDoor _outactors)
    (bind _outactors_2 (Actor|GetAllActorsOfClass "/Game/BluePrints/Doors/AppearingDoor.AppearingDoor_C"))
    (Default|AppearDoor _outactors_2)
    (Variables|Default|SetIsThirdDocumentRead true)))

(event Custom|PauseMenu:%20Go%20To%20Main%20Menu
  ;[1 1 1] Меню паузы: выход в главное меню
  (Utilities|IsValid (Variables|Widgets|GetPauseToMainMenu)
    (:Is%20Valid
      _)
    (:Is%20Not%20Valid
      (bind _returnvalue (UserInterface|CreateWidget "/Game/UI/Menus/PauseToMainMenuWB.PauseToMainMenuWB_C" (Game|GetPlayerController 0)))
      (Variables|Widgets|SetPauseToMainMenu _returnvalue)))
  (UserInterface|Viewport|AddtoViewport (Variables|Widgets|GetPauseToMainMenu) 0)
  (Widget|RemovefromParent (Variables|Widgets|GetPauseMenuWB)))

(event Custom|Pause%20Menu%20To%20Main%20Menu:%20Accept
  ;[1 1 1] Меню паузы: выход в главное меню
  (Game|OpenLevel(byObjectReference) "/Game/FirstPersonBP/Maps/MainMenu.MainMenu"))

(event Custom|Pause%20Menu%20To%20Main%20Menu:%20Decline
  ;[1 1 1] Меню паузы: выход в главное меню
  (Widget|RemovefromParent (Variables|Widgets|GetPauseToMainMenu))
  (UserInterface|Viewport|AddtoViewport (Variables|Widgets|GetPauseMenuWB) 0))

(event Custom|Show%20Inventory
  (bind _returnvalue (Game|GetPlayerController 0))
  ;[1 1 1] Вызов инвентаря
  (Utilities|IsValid (Variables|Widgets|GetInventoryWB)
    (:Is%20Valid
      _)
    (:Is%20Not%20Valid
      (bind _returnvalue_2 (UserInterface|CreateWidget "/Game/UI/Documents/Inventory.Inventory_C" _returnvalue))
      (Variables|Widgets|SetInventoryWB _returnvalue_2)))
  (UserInterface|Viewport|AddtoViewport (Variables|Widgets|GetInventoryWB) 0)
  (Input|SetInputModeUIOnly _returnvalue (Variables|Widgets|GetInventoryWB) "LockInFullscreen")
  (Game|SetGamePaused true)
  (Variables|/Script/Engine.PlayerController|SetbShowMouseCursor _returnvalue true))

(fn SetAngelatIndex
  (params (Index :type Integer) (IsCorrect :type Boolean))
  (Utilities|Array|SetArrayElem (Variables|Default|GetAngelsPositions) Index IsCorrect))

(fn IsAllAngelsCorrect
  (bind _angelspositions (Variables|Default|GetAngelsPositions))
  (return (Math|Boolean|ANDBoolean (Utilities|Array|Get(acopy) _angelspositions) (Utilities|Array|Get(acopy) _angelspositions 1) (Utilities|Array|Get(acopy) _angelspositions 2) (Utilities|Array|Get(acopy) _angelspositions 3) (Utilities|Array|Get(acopy) _angelspositions 4) (Utilities|Array|Get(acopy) _angelspositions 5))))