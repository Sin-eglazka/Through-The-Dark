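; End-game mirror actor that lets the player finish the game by interacting with it.
; The EndGame collision component starts disabled until EnableEvent turns it on, and a separate EditMaterial event swaps the mesh to an emissive material.
; Overlapping EndGame enables input and leaving disables it, so pressing E in range calls EndGameMirror on MainGameInstanse.
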(event OnComponentBeginOverlap(EndGame)
  (params (OverlappedComponent :type Primitive%20Component%20Object%20Reference) (OtherActor :type Actor%20Object%20Reference) (OtherComp :type Primitive%20Component%20Object%20Reference) (OtherBodyIndex :type Integer) (bFromSweep :type Boolean) (SweepResult :type Hit%20Result%20Structure%20%28by%20ref%29))
  (Input|EnableInput (Game|GetPlayerController 0)))

(event OnComponentEndOverlap(EndGame)
  (params (OverlappedComponent :type Primitive%20Component%20Object%20Reference) (OtherActor :type Actor%20Object%20Reference) (OtherComp :type Primitive%20Component%20Object%20Reference) (OtherBodyIndex :type Integer))
  (Input|DisableInput (Game|GetPlayerController 0)))

(event Custom|EnableEvent
  ;[1 1 1] Включение взаимодействия
  (Collision|SetCollisionEnabled (Variables|Default|GetEndGame) "QueryAndPhysics"))

(event Custom|EditMaterial
  ;[1 1 1] Сменить материал
  (Rendering|Material|SetMaterial (Variables|Debug|GetStaticMeshComponent) 0 "/Game/Materials/M_Opaque_MeshEmit_Emis_Master.M_Opaque_MeshEmit_Emis_Master"))

(event EventBeginPlay
  (Collision|SetCollisionEnabled (Variables|Default|GetEndGame) "NoCollision"))

(event Collision|EventActorBeginOverlap
  (params (OtherActor :type Actor%20Object%20Reference)))

(event EventTick
  (params (DeltaSeconds :type Float%20%28single-precision%29)))

(event Input|KeyboardEvents|E
  (params (Key :type Key%20Structure :default "None"))
  ;[1 1 1] Конец игры: Взаимодействие с зеркалом
  (:Pressed
    (bind _asmain_game_instanse (Utilities|Casting|CastToMainGameInstanse (Game|GetGameInstance)))
    (Default|EndGameMirror _asmain_game_instanse)))

(fn ConstructionScript)