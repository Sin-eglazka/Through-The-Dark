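; DiamondFind is a trigger Blueprint that lets the player destroy a mirror by pressing E while near it.
; On BeginPlay it casts and caches the MainGameInstanse game instance.
; Its Entering component enables input from player controller 0 on begin overlap and disables it on end overlap, without filtering the overlapping actor.
; The E press delegates the destruction to DestroyMirrow on the game instance.
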(event OnComponentBeginOverlap(Entering)
  (params (OverlappedComponent :type Primitive%20Component%20Object%20Reference) (OtherActor :type Actor%20Object%20Reference) (OtherComp :type Primitive%20Component%20Object%20Reference) (OtherBodyIndex :type Integer) (bFromSweep :type Boolean) (SweepResult :type Hit%20Result%20Structure%20%28by%20ref%29))
  ;[1 1 1] Включение ввода
  (Input|EnableInput (Game|GetPlayerController 0)))

(event OnComponentEndOverlap(Entering)
  (params (OverlappedComponent :type Primitive%20Component%20Object%20Reference) (OtherActor :type Actor%20Object%20Reference) (OtherComp :type Primitive%20Component%20Object%20Reference) (OtherBodyIndex :type Integer))
  ;[1 1 1] Включение ввода
  (Input|DisableInput (Game|GetPlayerController 0)))

(event EventBeginPlay
  (bind _asmain_game_instanse (Utilities|Casting|CastToMainGameInstanse (Game|GetGameInstance)))
  (Variables|Default|SetAs%20Main%20Game%20Instanse _asmain_game_instanse))

(event Collision|EventActorBeginOverlap
  (params (OtherActor :type Actor%20Object%20Reference)))

(event EventTick
  (params (DeltaSeconds :type Float%20%28single-precision%29)))

(event Input|KeyboardEvents|E
  (params (Key :type Key%20Structure))
  ;[1 1 1] Разрушение зеркала
  (:Pressed
    (Default|DestroyMirrow (Variables|Default|GetAs%20Main%20Game%20Instanse))))

(fn ConstructionScript)