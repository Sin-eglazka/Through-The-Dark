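; Door actor that swings open when the first-person character enters its trigger and closes when they leave.
; The DoorCollision trigger starts with collision off at BeginPlay, so the door stays inactive until SetDoorEnabled turns it on.
; Overlap events play or reverse the Open timeline, which scales the Angle variable into DoorOpen's relative yaw while holding a fixed roll.
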(event OnComponentBeginOverlap(DoorCollision)
  (params (OverlappedComponent :type Primitive%20Component%20Object%20Reference) (OtherActor :type Actor%20Object%20Reference) (OtherComp :type Primitive%20Component%20Object%20Reference) (OtherBodyIndex :type Integer) (bFromSweep :type Boolean) (SweepResult :type Hit%20Result%20Structure%20%28by%20ref%29))
  ;[1 1 1] Открытие и закрытие двери
  (Utilities|Casting|CastToFirstPersonCharacter OtherActor)
  (bind _opening (Timeline|Open Play)
    (:Update
      (Transformation|SetRelativeRotation (Variables|Default|GetDoorOpen) (Math|Rotator|MakeRotator -9e+01 0.0 (* _opening (Variables|Default|GetAngle))) false false))))

(event OnComponentEndOverlap(DoorCollision)
  (params (OverlappedComponent :type Primitive%20Component%20Object%20Reference) (OtherActor :type Actor%20Object%20Reference) (OtherComp :type Primitive%20Component%20Object%20Reference) (OtherBodyIndex :type Integer))
  ;[1 1 1] Открытие и закрытие двери
  (Utilities|Casting|CastToFirstPersonCharacter OtherActor)
  (bind _opening (Timeline|Open Reverse)
    (:Update
      (Transformation|SetRelativeRotation (Variables|Default|GetDoorOpen) (Math|Rotator|MakeRotator -9e+01 0.0 (* _opening (Variables|Default|GetAngle))) false false))))

(event Custom|SetDoorEnabled
  (Collision|SetCollisionEnabled (Variables|Default|GetDoorCollision) "QueryAndPhysics"))

(event EventBeginPlay
  (Collision|SetCollisionEnabled (Variables|Default|GetDoorCollision) "NoCollision"))

(event Collision|EventActorBeginOverlap
  (params (OtherActor :type Actor%20Object%20Reference)))

(event EventTick
  (params (DeltaSeconds :type Float%20%28single-precision%29)))

(fn ConstructionScript)