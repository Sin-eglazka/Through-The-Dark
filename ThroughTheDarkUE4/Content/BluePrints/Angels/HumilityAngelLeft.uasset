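; Left Humility angel statue for a puzzle: pressing E inside the Smirenie1 overlap zone slides it along world X.
; A timeline moves the mesh each update, while a signed Scale counter tracks position and reverses direction after every two moves.
; After each move, it reports whether it is correctly placed to MainGameInstanse at index 2 and triggers the all-angels check.
; Once all angels are correct, pressing E disables the zone's collision instead.
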(event OnComponentBeginOverlap(Smirenie1)
  (params (OverlappedComponent :type Primitive%20Component%20Object%20Reference) (OtherActor :type Actor%20Object%20Reference) (OtherComp :type Primitive%20Component%20Object%20Reference) (OtherBodyIndex :type Integer) (bFromSweep :type Boolean) (SweepResult :type Hit%20Result%20Structure%20%28by%20ref%29))
  (Input|EnableInput (Game|GetPlayerController 0)))

(event OnComponentEndOverlap(Smirenie1)
  (params (OverlappedComponent :type Primitive%20Component%20Object%20Reference) (OtherActor :type Actor%20Object%20Reference) (OtherComp :type Primitive%20Component%20Object%20Reference) (OtherBodyIndex :type Integer))
  (Input|DisableInput (Game|GetPlayerController 0)))

(event Custom|SetPosition
  (bind _as_main_game_instanse (Variables|Default|GetAs%20Main%20Game%20Instanse))
  ;[1 1 1] Проверка на корректное расположение
  (bind _iscorrect (CallFunction|IsCorrectPosition))
  (Default|SetAngelatIndex _as_main_game_instanse 2 _iscorrect)
  (Default|AllAngelsCorrect _as_main_game_instanse))

(event EventBeginPlay
  (bind _asmain_game_instanse (Utilities|Casting|CastToMainGameInstanse (Game|GetGameInstance)))
  (Variables|Default|SetAs%20Main%20Game%20Instanse _asmain_game_instanse))

(event Collision|EventActorBeginOverlap
  (params (OtherActor :type Actor%20Object%20Reference)))

(event EventTick
  (params (DeltaSeconds :type Float%20%28single-precision%29)))

(event Input|KeyboardEvents|E
  (params (Key :type Key%20Structure :default "None"))
  (bind _staticmeshcomponent (Variables|Debug|GetStaticMeshComponent))
  (bind _returnvalue (Transformation|GetWorldLocation _staticmeshcomponent))
  (:Pressed
    (bind _iscorrect (Default|IsAllAngelsCorrect (Variables|Default|GetAs%20Main%20Game%20Instanse)))
    (if _iscorrect
      (Collision|SetCollisionEnabled (Variables|Default|GetSmirenie1) "NoCollision")
      (elif (not (Variables|Default|GetIsMoving))
        (Default|PlayAngelSound (Variables|Default|GetAs%20Main%20Game%20Instanse))
        ;[1 1 1] Передвижение объекта
        (Variables|Default|SetIsMoving true)
        (if (> (Variables|Default|GetScale) 0.0)
          (Variables|Default|SetWay 1.0)
          (Timeline|Timeline_0 PlayFromStart
            (:Update
              (Transformation|SetWorldLocation (Variables|Debug|GetStaticMeshComponent) (Math|Vector|MakeVector (+ (Variables|Default|GetWay) (.x _returnvalue)) (.y _returnvalue) (.z _returnvalue)) false false))
            (:Finished
              ;[1 1 1] Изменение шкалы положения
              (if (> (Variables|Default|GetScale) 0.0)
                (bind _output_get (Variables|Default|SetScale (+ (Variables|Default|GetScale) 1.0)))
                (if (== _output_get 3.0)
                  (Variables|Default|SetScale -1.0))
                (else
                  (bind _output_get_2 (Variables|Default|SetScale (- (Variables|Default|GetScale) 1.0)))
                  (if (== _output_get_2 -3.0)
                    (Variables|Default|SetScale 1.0))))
              (CallFunction|SetPosition)
              (Variables|Default|SetIsMoving false)))
          (else
            (Variables|Default|SetWay -1.0)
            (Timeline|Timeline_0 PlayFromStart)))))))

(fn ConstructionScript)

(fn IsCorrectPosition
  (return (== (Variables|Default|GetScale) -1.0)))